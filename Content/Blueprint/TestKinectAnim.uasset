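; Test actor, named for Kinect animation, that pairs a skeletal mesh with a bone-following camera offset and a physics poke on one arm.
; Each tick it moves CameraOffset to the neck_01 socket location in actor space, following position only.
; Space bar sets a physics angular velocity on the left upper arm bone.
; No Kinect input appears in the graph, and a clavicle rotation debug print is left unconnected.
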(event `self.ReceiveEndPlay`
  (params (EndPlayReason :type "EEndPlayReason Enum" :default "Destroyed")))

(event `self.ReceiveTick`
  (params (DeltaSeconds :type "Float (single-precision)"))
  (`SceneComponent.K2_SetRelativeLocation` (`self.CameraOffset`) (.location (`SceneComponent.GetSocketTransform` (`self.SkeletalMesh`) "neck_01" "RTS_Actor")) false false))

(event `Key|SpaceBar`
  (params (Key :type "Key Structure" :default "LeapLeftPinch"))
  (:`Pressed`
    (`PrimitiveComponent.SetPhysicsAngularVelocity` (`self.SkeletalMesh`) (0.0 33.0 0.0) false "upperarm_l")))

(fn `UserConstructionScript`)